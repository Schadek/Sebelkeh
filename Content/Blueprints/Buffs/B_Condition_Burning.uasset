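; Burning condition buff that damages a target over time by lowering its health regeneration.
; On begin it caches the target's StatComponent.
; Activate subtracts the Degeneration value from HealthRegeneration, and Deactivate adds the same value back to undo the effect.
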(event `self.ReceiveBegin`
  (params (_Target :type "Actor Object Reference") (_Instigator :type "Actor Object Reference") (_Duration :type "Float (single-precision)") (_bIsInfinite :type Boolean))
  (set `self.StatComponent` (`Actor.GetComponentByClass` _Target "/Script/CourtOfSebelkeh.StatComponent")))

(event `self.ReceiveActivate`
  (`StatComponent.AddStat` (`self.StatComponent`) "HealthRegeneration" (* (`self.Degeneration`) -1)))

(event `self.ReceiveDeactivate`
  (`StatComponent.AddStat` (`self.StatComponent`) "HealthRegeneration" (`self.Degeneration`)))