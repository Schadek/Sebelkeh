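; TargetPractice is an actor with a mesh and floating name label, apparently a selectable practice target.
; Selectable hover delegates toggle the mesh's custom depth rendering, typically used for highlight outlines.
; ActorMeta supplies the label text on BeginPlay and updates it through its name-changed delegate.
; Every tick, the TextRender rotates to face the player camera, using the direction from the actor's location.
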(event `self.Selectable.OnHoverBeginDel`
  (params (SelectableComponent :type "SelectableComponent Object Reference") (Controller :type "PlayerController Object Reference"))
  (`PrimitiveComponent.SetRenderCustomDepth` (`self.Mesh`) true))

(event `self.Selectable.OnHoverEndDel`
  (params (SelectableComponent :type "SelectableComponent Object Reference") (Controller :type "PlayerController Object Reference"))
  (`PrimitiveComponent.SetRenderCustomDepth` (`self.Mesh`) false))

(event `self.ActorMeta.OnNameChangedDel`
  (params (Component :type "ActorMetaComponent Object Reference") (NewName :type "Text (by ref)"))
  (`TextRenderComponent.K2_SetText` (`self.TextRender`) NewName))

(event `self.ReceiveBeginPlay`
  (`TextRenderComponent.K2_SetText` (`self.TextRender`) (`ActorMetaComponent.GetName` (`self.ActorMeta`))))

(event `self.ReceiveTick`
  (params (DeltaSeconds :type "Float (single-precision)"))
  (bind _returnvalue (`GameplayStatics.GetPlayerCameraManager` 0))
  (`/Engine/EditorBlueprintResources/StandardMacros.IsValid` _returnvalue
    (:`Is Valid`
      (`SceneComponent.K2_SetWorldRotation` (`self.TextRender`) (`KismetMathLibrary.MakeRotFromX` (- (`PlayerCameraManager.GetCameraLocation` _returnvalue) (`self.K2_GetActorLocation`))) false false))))

(fn `UserConstructionScript`)