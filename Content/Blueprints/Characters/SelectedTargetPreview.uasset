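; Preview actor that renders the player's selected target through a scene capture, mirroring that target's skeletal mesh.
; It listens for target changes on the CorePlayerController and reads the new target owner's mesh and ActorMetaComponent.
; If the preview mesh's current skeleton has the meta's camera socket, it swaps meshes, enables per-frame capture and positions the spring arm there at the meta's distance.
; Otherwise per-frame capture stops.
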(event `self.ReceiveBeginPlay`
  (bind _ascore_player_controller (cast `CorePlayerController` (`GameplayStatics.GetPlayerController` 0)))
  (add `CorePlayerController.OnSelectedTargetChanged` _ascore_player_controller (delegate `OnSelectedTargetChanged`)))

(event `OnSelectedTargetChanged`
  (params (Controller :type "CorePlayerController Object Reference") (OldTarget :type "SelectableComponent Object Reference") (NewTarget :type "SelectableComponent Object Reference"))
  (bind _returnvalue (`ActorComponent.GetOwner` NewTarget))
  (`/Engine/EditorBlueprintResources/StandardMacros.IsValid` NewTarget
    (:`Is Valid`
      (bind _output_get (set `self.CurrentSkeletalMeshComponent` (`self.GetComponentByClass` _returnvalue "/Script/Engine.SkeletalMeshComponent")))
      (`self.SetPreviewCharacter` (`SkinnedMeshComponent.SkeletalMesh` _output_get) (`self.GetComponentByClass` _returnvalue "/Script/CourtOfSebelkeh.ActorMetaComponent")))))

(fn `SetPreviewCharacter`
  (params (SkeletalMesh :type "SkeletalMesh Object Reference") (Meta :type "ActorMetaComponent Object Reference"))
  (bind _returnvalue (`ActorMetaComponent.GetTargetPreviewCameraSocket` Meta))
  (bind _skeletalmesh1 (`self.SkeletalMesh1`))
  (`/Engine/EditorBlueprintResources/StandardMacros.IsValid` Meta
    (:`Is Valid`
      (if (`SceneComponent.DoesSocketExist` _skeletalmesh1 _returnvalue)
        (`SkinnedMeshComponent.SetSkinnedAssetAndUpdate` (`self.SkeletalMesh1`) SkeletalMesh false)
        (set `SceneCaptureComponent.bCaptureEveryFrame` true (`self.SceneCaptureComponent2D`))
        (`SceneComponent.K2_SetWorldLocation` (`self.SpringArm`) (`SceneComponent.GetSocketLocation` _skeletalmesh1 _returnvalue) false false)
        (set `SpringArmComponent.TargetArmLength` (`ActorMetaComponent.GetTargetPreviewCameraDistance` Meta) (`self.SpringArm`))
        (else
          (set `SceneCaptureComponent.bCaptureEveryFrame` false (`self.SceneCaptureComponent2D`) :!label _label))))
    (:`Is Not Valid`
      (goto _label))))

(fn `UserConstructionScript`)