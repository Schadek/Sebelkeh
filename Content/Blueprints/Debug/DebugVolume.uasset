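; DebugVolume is a debug actor that displays a configurable text label in the world.
; The construction script applies the Text and TextSize variables to its TextRender component.
; Each Tick rotates the label toward the first player's camera, billboard-style, using the direction from the actor's location to the camera.
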(event `self.ReceiveTick`
  (params (DeltaSeconds :type "Float (single-precision)"))
  (bind _returnvalue (`GameplayStatics.GetPlayerCameraManager` 0))
  (`/Engine/EditorBlueprintResources/StandardMacros.IsValid` _returnvalue
    (:`Is Valid`
      (`SceneComponent.K2_SetWorldRotation` (`self.TextRender`) (`KismetMathLibrary.MakeRotFromX` (- (`PlayerCameraManager.GetCameraLocation` _returnvalue) (`self.K2_GetActorLocation`))) false false))))

(fn `UserConstructionScript`
  (bind _textrender (`self.TextRender`))
  (`TextRenderComponent.K2_SetText` _textrender (`self.Text`))
  (`TextRenderComponent.SetWorldSize` _textrender (`self.TextSize`)))